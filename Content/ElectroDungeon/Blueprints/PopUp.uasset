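; PopUp is an enemy or hazard actor that hurts the player on contact and can be destroyed by damage.
; When its Box overlaps a Player_Idle_Blueprint, it calls that player's DamageSystem with a small fixed amount, noted as damage to the phone.
; The PopUp_Gets_DMG event, meant for bullet hits, subtracts from PopUpHealth, destroys the actor at zero or below, and otherwise prints the remaining health.
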(event OnComponentBeginOverlap(Box)
  (params (OverlappedComponent :type Primitive%20Component%20Object%20Reference) (OtherActor :type Actor%20Object%20Reference) (OtherComp :type Primitive%20Component%20Object%20Reference) (OtherBodyIndex :type Integer) (bFromSweep :type Boolean) (SweepResult :type Hit%20Result%20Structure%20%28by%20ref%29))
  ;[1 1 1] Apply Damage to Phone
  (bind _asplayer_idle_blueprint (Utilities|Casting|CastToPlayer_Idle_Blueprint OtherActor))
  (Default|DamageSystem _asplayer_idle_blueprint 0.05))

(event Custom|PopUp_Gets_DMG
  (params (DMGTaken :type Integer))
  ;[1 1 1] Take Damage from Bullet
  (bind _output_get (Variables|Default|SetPopUp_Health (- (Variables|Default|GetPopUp_Health) DMGTaken)))
  (if (<= _output_get 0)
    (Actor|DestroyActor)
    (else
      (Development|PrintString (Utilities|String|ToString(Integer) (Variables|Default|GetPopUp_Health))))))

(event EventBeginPlay)

(event Collision|EventActorBeginOverlap
  (params (OtherActor :type Actor%20Object%20Reference)))

(event EventTick
  (params (DeltaSeconds :type Float%20%28single-precision%29)))

(fn ConstructionScript)