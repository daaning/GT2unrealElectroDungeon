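; Akkufresser is an enemy actor that chases the Paper2D player and damages their phone through DamageSystem when its box begins overlapping them.
; Each Tick it turns to face the player and steps toward them in X and Z at a fixed per-frame speed, regardless of distance.
; Incoming damage lowers its health; at zero it destroys itself and notifies the DestroyedEnemiesCounter.
; An older range-based follow remains as disconnected nodes.
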(event OnComponentBeginOverlap(Box)
  (params (OverlappedComponent :type Primitive%20Component%20Object%20Reference) (OtherActor :type Actor%20Object%20Reference) (OtherComp :type Primitive%20Component%20Object%20Reference) (OtherBodyIndex :type Integer) (bFromSweep :type Boolean) (SweepResult :type Hit%20Result%20Structure%20%28by%20ref%29))
  ;[1 1 1] Apply Damage to Phone
  (bind _asplayer_idle_blueprint (Utilities|Casting|CastToPlayer_Idle_Blueprint OtherActor))
  (Default|DamageSystem _asplayer_idle_blueprint 0.1))

(event Custom|Akkufresser_Gets_DMG
  (params (DMGTaken :type Integer))
  ;[1 1 1] Take Damage from Bullet
  (bind _output_get (Variables|Default|SetAkkufresser_Health (- (Variables|Default|GetAkkufresser_Health) DMGTaken)))
  (if (<= _output_get 0)
    (Actor|DestroyActor)
    (bind _outactors (Actor|GetAllActorsOfClass "/Game/ElectroDungeon/Blueprints/DestroyedEnemiesCounter.DestroyedEnemiesCounter_C"))
    (Default|EnemyDestroyed (Utilities|Array|Get(acopy) _outactors))))

(event EventTick
  (params (DeltaSeconds :type Float%20%28single-precision%29))
  (bind _returnvalue (Transformation|GetActorLocation))
  (bind _returnvalue_2 (Transformation|GetActorLocation))
  (bind _returnvalue_3 (Game|GetPlayerCharacter 0))
  (bind _returnvalue_4 (Transformation|GetActorLocation _returnvalue_3))
  (bind _returnvalue_5 (Math|Rotator|FindLookatRotation _returnvalue_2 _returnvalue_4))
  (Utilities|FlowControl|Sequence
    (:then_0
      (bind _output_get (Variables|Default|SetDistance (- (.X (Math|Vector|BreakVector (Transformation|GetWorldLocation (Variables|Default|GetAkkufresser)))) (.X (Math|Vector|BreakVector (Transformation|GetActorLocation (Game|GetPlayerCharacter 0)))))))
      (if (<= _output_get 4e+02)
        _))
    (:then_1
      (Transformation|SetActorRotation (Math|Rotator|MakeRotator (.roll _returnvalue_5) (.pitch _returnvalue_5) (.yaw _returnvalue_5))))
    (:then_2
      ;[1 1 1] Follow2
      (Variables|Default|SetFresserX (.x _returnvalue))
      (Variables|Default|SetFresserY (.y _returnvalue))
      (Variables|Default|SetFresserZ (.z _returnvalue))
      (bind _aspaper_character (Utilities|Casting|CastToPaperCharacter (Game|GetPlayerCharacter 0)))
      (bind _asplayer_idle_blueprint (Utilities|Casting|CastToPlayer_Idle_Blueprint _aspaper_character))
      (bind _returnvalue_6 (Default|GetPlayerLocation _asplayer_idle_blueprint))
      (Variables|Default|SetPlayerX (.x _returnvalue_6))
      (Variables|Default|SetPlayerZ (.z _returnvalue_6))
      (Variables|Default|SetMoveSpeed 0.7)
      (Transformation|SetActorLocation (Math|Vector|MakeVector (+ (Variables|Default|GetFresserX) (* (Math|Float|Sign(Float) (- (Variables|Default|GetPlayerX) (Variables|Default|GetFresserX))) (Variables|Default|GetMoveSpeed))) (Variables|Default|GetFresserY) (+ (* (Variables|Default|GetMoveSpeed) (Math|Float|Sign(Float) (- (Variables|Default|GetPlayerZ) (Variables|Default|GetFresserZ)))) (Variables|Default|GetFresserZ))) false false))))

(fn ConstructionScript)