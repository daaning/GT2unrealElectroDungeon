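; TempPrint is a Blueprint holding a disconnected "Follow2" chase snippet for a Fresser actor; nothing in it runs.
; The snippet gets the player's location through Player_Idle_Blueprint and steps the actor toward it by a fixed amount on X and Z, keeping Y unchanged.
; Movement uses the sign of each axis difference, with no delta-time scaling.
; The construction script is empty.
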(fn ConstructionScript)