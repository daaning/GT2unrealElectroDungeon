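; Player pawn for a 2D Paper2D game where health acts as a battery that drains every second.
; Axis inputs move it in the XZ plane, while Tick picks a directional or idle flipbook from velocity and last input direction.
; Left click spawns BP_Bullet aimed at the deprojected cursor.
; DamageSystem and Charge adjust health, but zero checks drive nothing and Charge's cap compares constants, so never fires.
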(event Custom|Damage%20System
  (params (DmgOut :type Float%20%28single-precision%29))
  ;[1 1 1] Damage
  (bind _output_get (Variables|Default|SetPlayer_Health (- (Variables|Default|GetPlayer_Health) DmgOut)))
  (Math|Float|CompareFloat _output_get 0.0) ; compare to zero
)

(event Custom|Charge
  (params (Charge :type Float%20%28single-precision%29))
  ;[1 1 1] Charge
  (Variables|Default|SetPlayer_Health (+ (Variables|Default|GetPlayer_Health) Charge))
  (Math|Float|CompareFloat 0.0 1.0
    (:>
      (Variables|Default|SetPlayer_Health 1.0))))

(event Custom|LessEverySecond
  ;[1 1 1] Lose Battery every seocond
  (bind _output_get (Variables|Default|SetPlayer_Health (- (Variables|Default|GetPlayer_Health) 0.01)))
  (Math|Float|CompareFloat _output_get 0.0) ; compare to zero
)

(event EventBeginPlay
  (Utilities|FlowControl|Sequence
    (:then_0
      ;[1 1 1] Add UI to Screen
      (bind _returnvalue (UserInterface|CreateWidget "/Game/ElectroDungeon/UI/InGameUI.InGameUI_C"))
      (UserInterface|Viewport|AddtoViewport _returnvalue 0))
    (:then_1
      ;[1 1 1] Replication
      (Class|ActorComponent|SetIsReplicated (Variables|Default|GetSprite) false) ; for multiplayer that i wont have
    )
    (:then_2
      (Utilities|Time|SetTimerbyFunctionName 0 "LessEverySecond" 1.0 true))))

(event EventTick
  (params (DeltaSeconds :type Float%20%28single-precision%29))
  ;[1 1 1] Animation
  (CallFunction|SetCorrectFlipbook))

(event Input|AxisEvents|InputAxisMove_Left_Right
  (params (AxisValue :type Float%20%28single-precision%29))
  ;[1 1 1] Movement Left Right
  (Pawn|Input|AddMovementInput "1.000000,0.000000, 0" AxisValue false))

(event Input|AxisEvents|InputAxisMove_Up_Down
  (params (AxisValue :type Float%20%28single-precision%29))
  ;[1 1 1] Movement Up Down
  (Pawn|Input|AddMovementInput "0.000000,0.000000,1.000000" AxisValue false))

(event Input|MouseEvents|LeftMouseButton
  (params (Key :type Key%20Structure :default "None"))
  (bind _returnvalue (Game|GetPlayerController 0))
  (bind _returnvalue_2 (Pawn|GetControlledPawn _returnvalue))
  (bind _worldlocation (Game|Player|ConvertMouseLocationToWorldSpace _returnvalue))
  (bind _returnvalue_3 (Transformation|GetActorLocation _returnvalue_2))
  (bind (_x _y _z) (Math|Vector|BreakVector _worldlocation))
  (bind _returnvalue_4 (Math|Vector|MakeVector _x 0.0 _z))
  (bind _returnvalue_5 (Math|Rotator|FindLookatRotation _returnvalue_3 _returnvalue_4))
  ;[1 1 1] Shooting at Cursor
  (:Pressed
    (Game|SpawnActorfromClass "/Game/ElectroDungeon/Blueprints/BP_Bullet.BP_Bullet_C" (Math|Transform|MakeTransform (+ _returnvalue_3 (Math|Vector|GetForwardVector _returnvalue_5)) _returnvalue_5) "Undefined" 0 0)))

(fn ConstructionScript)

(fn SetCorrectFlipbook
  (if (or (!= (Input|AxisValues|GetMove_Up_Down) 0.0) (!= (Input|AxisValues|GetMove_Left_Right) 0.0))
    (Variables|Default|SetLastMoveDirection (select (> (Input|AxisValues|GetMove_Up_Down) 0.0) "NewEnumerator0" (select (< (Input|AxisValues|GetMove_Up_Down) 0.0) "NewEnumerator1" (select (> (Input|AxisValues|GetMove_Left_Right) 0.0) "NewEnumerator3" "NewEnumerator2")))) ; Which animation should we choose?
  )
  (Sprite|SetFlipbook (Variables|Default|GetSprite) (select (> (Math|Vector|VectorLength (Transformation|GetVelocity)) 0.0) (Utilities|Select :Index (Variables|Default|GetLastMoveDirection) :NewEnumerator0 "/Game/ElectroDungeon/Sprites/Player_Up.Player_Up" :NewEnumerator1 "/Game/ElectroDungeon/Sprites/Player_Forward.Player_Forward" :NewEnumerator2 "/Game/ElectroDungeon/Sprites/Player_left.Player_Left" :NewEnumerator3 "/Game/ElectroDungeon/Sprites/Player_Right.Player_Right") (Utilities|Select :Index (Variables|Default|GetLastMoveDirection) :NewEnumerator0 "/Game/ElectroDungeon/Sprites/Player_Idle.Player_Idle" :NewEnumerator1 "/Game/ElectroDungeon/Sprites/Player_Idle.Player_Idle" :NewEnumerator2 "/Game/ElectroDungeon/Sprites/Player_Idle.Player_Idle" :NewEnumerator3 "/Game/ElectroDungeon/Sprites/Player_Idle.Player_Idle"))))

(fn GetPlayerLocation
  (return (Transformation|GetActorLocation (Pawn|GetControlledPawn (Game|GetPlayerController 0)))))