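; Paper2D boss enemy that creeps toward the player in X and Z by a fixed step each Tick and damages them on box overlap.
; A six-second looping timer randomly switches its flipbook between intro and jump through AnimStateMachine, leaving idle unused.
; Boss_Gets_DMG drains health, then at zero plays the death flipbook and opens the Win level without waiting for the delayed destroy.
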(event OnComponentBeginOverlap(Box)
  (params (OverlappedComponent :type Primitive%20Component%20Object%20Reference) (OtherActor :type Actor%20Object%20Reference) (OtherComp :type Primitive%20Component%20Object%20Reference) (OtherBodyIndex :type Integer) (bFromSweep :type Boolean) (SweepResult :type Hit%20Result%20Structure%20%28by%20ref%29))
  ;[1 1 1] Apply Damage to Phone
  (bind _asplayer_idle_blueprint (Utilities|Casting|CastToPlayer_Idle_Blueprint OtherActor))
  (Default|DamageSystem _asplayer_idle_blueprint 0.1))

(event Custom|Boss_Gets_DMG
  (params (DMGTaken :type Integer))
  ;[1 1 1] Take Damage from Bullet
  (bind _output_get (Variables|Default|SetBoss_Health (- (Variables|Default|GetBoss_Health) DMGTaken)))
  (if (<= _output_get 0)
    (Utilities|FlowControl|Sequence
      (:then_0
        (Sprite|SetFlipbook (Variables|Default|GetBoss) "/Game/ElectroDungeon/Sprites/Boss_Death.Boss_Death")
        (Utilities|FlowControl|Delay 5.0)
        (Actor|DestroyActor))
      (:then_1
        (Game|OpenLevel(byName) "Win")))))

(event Custom|UpdateAnimation
  ;[1 1 1] Animation
  (Utilities|FlowControl|Sequence
    (:then_0
      ;;[1 1 1] Get random value every time function is called
      (Variables|Default|SetisMoving (Math|Random|RandomBool)))
    (:then_1
      ;;[1 1 1] Set Paper Flipbook depending on random bool
      (bind _output_get (Variables|Default|SetisMoving (Variables|Default|GetisMoving)))
      (bind _output_flipbook (CallFunction|AnimStateMachine _output_get))
      (Sprite|SetFlipbook (Variables|Default|GetBoss) _output_flipbook))))

(event EventBeginPlay
  ;[1 1 1] Animation
  (Utilities|Time|SetTimerbyFunctionName 0 "UpdateAnimation" 6.0 true))

(event Collision|EventActorBeginOverlap
  (params (OtherActor :type Actor%20Object%20Reference)))

(event EventTick
  (params (DeltaSeconds :type Float%20%28single-precision%29))
  (bind _returnvalue (Transformation|GetActorLocation))
  (Utilities|FlowControl|Sequence
    (:then_0
      (bind _output_get (Variables|Default|SetDistance (- (.X (Math|Vector|BreakVector (Transformation|GetWorldLocation (Variables|Default|GetBoss)))) (.X (Math|Vector|BreakVector (Transformation|GetActorLocation (Game|GetPlayerCharacter 0)))))))
      (if (<= _output_get 4e+02)
        _))
    (:then_1
      ;[1 1 1] Follow2
      (Variables|Default|SetFresserX (.x _returnvalue))
      (Variables|Default|SetFresserY (.y _returnvalue))
      (Variables|Default|SetFresserZ (.z _returnvalue))
      (bind _aspaper_character (Utilities|Casting|CastToPaperCharacter (Game|GetPlayerCharacter 0)))
      (bind _asplayer_idle_blueprint (Utilities|Casting|CastToPlayer_Idle_Blueprint _aspaper_character))
      (bind _returnvalue_2 (Default|GetPlayerLocation _asplayer_idle_blueprint))
      (Variables|Default|SetPlayerX (.x _returnvalue_2))
      (Variables|Default|SetPlayerZ (.z _returnvalue_2))
      (Variables|Default|SetMoveSpeed 0.3)
      (Transformation|SetActorLocation (Math|Vector|MakeVector (+ (Variables|Default|GetFresserX) (* (Math|Float|Sign(Float) (- (Variables|Default|GetPlayerX) (Variables|Default|GetFresserX))) (Variables|Default|GetMoveSpeed))) (Variables|Default|GetFresserY) (+ (* (Variables|Default|GetMoveSpeed) (Math|Float|Sign(Float) (- (Variables|Default|GetPlayerZ) (Variables|Default|GetFresserZ)))) (Variables|Default|GetFresserZ))) false false))))

(fn ConstructionScript)

(fn AnimStateMachine
  (params (IsMoving :type Boolean))
  (Variables|Animations|SetAnimationState "NewEnumerator2")
  (if IsMoving
    (Variables|Animations|SetAnimationState "NewEnumerator1")
    (else
      (Variables|Animations|SetAnimationState "NewEnumerator3")))
  (return (Utilities|Select :Index (Variables|Animations|GetAnimationState) :NewEnumerator1 (Variables|Animations|GetBoss_Intro) :NewEnumerator2 (Variables|Animations|GetBoss_Idle) :NewEnumerator3 (Variables|Animations|GetBoss_Jump))))